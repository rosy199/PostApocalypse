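; Scene capture actor for snow trails that follows the player and accumulates its capture into a persistent render target.
; Each tick it moves in XY to the player's position, snapped to the capture's pixel grid to avoid sub-texel drift.
; It publishes size and location to MPC_Capture, then draws M_CopyToPersistent into RT_CapturePersistent, passing the normalized move offset so trails can stay world-aligned.
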(event `self.ReceiveBeginPlay`
  (`KismetMaterialLibrary.SetScalarParameterValue` "/Game/Snow/SnowTrail/MPC_Capture.MPC_Capture" "CaptureSize" (`SceneCaptureComponent2D.OrthoWidth` (`self.SceneCaptureComponent2D`)))
  (bind _returnvalue (`KismetMaterialLibrary.CreateDynamicMaterialInstance` "/Game/Snow/SnowTrail/M_CopyToPersistent.M_CopyToPersistent"))
  (set `self.Draw Material` _returnvalue)
  (`KismetRenderingLibrary.ClearRenderTarget2D` "/Game/Snow/SnowTrail/RT_Capture.RT_Capture")
  (`KismetRenderingLibrary.ClearRenderTarget2D` "/Game/Snow/SnowTrail/RT_CapturePersistent.RT_CapturePersistent"))

(event `self.ReceiveTick`
  (params (DeltaSeconds :type "Float (single-precision)"))
  (`self.MoveCapture`)
  (`self.DrawToPersistent`))

(fn `DrawToPersistent`
  (bind (_returnvalue_x _returnvalue_y) (`KismetMathLibrary.BreakVector2D` (/ (`self.MoveOffset`) (`SceneCaptureComponent2D.OrthoWidth` (`self.SceneCaptureComponent2D`)))))
  (`MaterialInstanceDynamic.SetVectorParameterValue` (`self.Draw Material`) "Offset" (make `LinearColor` _returnvalue_x _returnvalue_y 0.0 1.0))
  (`KismetRenderingLibrary.DrawMaterialToRenderTarget` "/Game/Snow/SnowTrail/RT_CapturePersistent.RT_CapturePersistent" (`self.Draw Material`)))

(fn `MoveCapture`
  (bind (_returnvalue_x _returnvalue_y) (`KismetMathLibrary.BreakVector` (`self.K2_GetActorLocation` (`GameplayStatics.GetPlayerCharacter` 0))))
  (bind _returnvalue (`KismetMaterialLibrary.GetScalarParameterValue` "/Game/Snow/SnowTrail/MPC_Capture.MPC_Capture" "CaptureSize"))
  (bind (_returnvalue_x_2 _returnvalue_y_2) (`KismetMathLibrary.BreakVector` (- (`self.SnapPixelToGrid` _returnvalue_x _returnvalue_y (* _returnvalue (/ 1.0 256.0))) (`self.K2_GetActorLocation`))))
  (bind _output_get (set `self.MoveOffset` (`KismetMathLibrary.MakeVector2D` _returnvalue_x_2 _returnvalue_y_2)))
  (`self.K2_AddActorWorldOffset` (`KismetMathLibrary.MakeVector` (`KismetMathLibrary.BreakVector2D` _output_get) (`.Y` (`KismetMathLibrary.BreakVector2D` _output_get))))
  (`KismetMaterialLibrary.SetVectorParameterValue` "/Game/Snow/SnowTrail/MPC_Capture.MPC_Capture" "CaptureLocation" (`KismetMathLibrary.Conv_VectorToLinearColor` (`self.K2_GetActorLocation`))))

(fn `UserConstructionScript`)